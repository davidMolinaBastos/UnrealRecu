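; Elevator actor that moves itself up and down continuously between its starting height and that height plus a configurable height difference.
; BeginPlay stores and prints both Z limits, then Tick uses the sign of Speed to pick which limit to check, flipping it on arrival.
; SetSpeed computes each new location by adding delta seconds plus Speed to Z, rather than multiplying them, so movement is a per-frame step.
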(event EventBeginPlay
  ;[1 0.8173 0] SetVariables
  (bind _output_get (Variables|Default|SetOriginalZ (.Z (Math|Vector|BreakVector (Transformation|GetActorLocation)))))
  (bind _output_get_2 (Variables|Default|SetFinalZ (+ _output_get (Variables|Default|GetHeightDiference))))
  (Development|PrintString (Utilities|String|ToString(Float) _output_get_2))
  (Development|PrintString (Utilities|String|ToString(Float) (Variables|Default|GetOriginalZ))))

(event Collision|EventActorBeginOverlap
  (params (OtherActor :type Actor%20Object%20Reference)))

(event EventTick
  (params (DeltaSeconds :type Float%20%28single-precision%29))
  ;[0 0.7366 1] Move Platform
  (if (> (Variables|Default|GetSpeed) 0.0)
    (if (< (.Z (Math|Vector|BreakVector (Transformation|GetActorLocation))) (Variables|Default|GetFinalZ))
      (bind _trans (CallFunction|SetSpeed (Variables|Default|GetSpeed) :!label _label))
      (Transformation|SetActorLocation _trans false false)
      (else
        (Utilities|InvertSpeed)))
    (elif (> (.Z (Math|Vector|BreakVector (Transformation|GetActorLocation))) (Variables|Default|GetOriginalZ))
      (goto _label)
      (else
        (Utilities|InvertSpeed)))))

(fn ConstructionScript)

(fn SetSpeed
  (params (Speed :type Float%20%28single-precision%29))
  (return (+ (Transformation|GetActorLocation) (Math|Vector|MakeVector 0.0 0.0 (+ (Utilities|Time|GetWorldDeltaSeconds) Speed)))))