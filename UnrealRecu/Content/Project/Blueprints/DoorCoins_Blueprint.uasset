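; A door Blueprint that responds to the player only once the character holds a minimum number of coins.
; On BeginPlay it shows MinCoins on its Number text.
; On overlap by a Player-tagged actor it compares Character.Coins with MinCoins and passes the event to the parent class only if the count suffices.
; An unconnected DoorCoin widget creation remains in the graph.
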(event EventBeginPlay
  ;[1 1 1] SetWidget
  (Rendering|Components|TextRender|SetText (Variables|Default|GetNumber) (Utilities|Text|ToText(Integer) (Variables|Default|GetMinCoins)))
  (|CallParentFunction))

(event Collision|EventActorBeginOverlap
  (params (OtherActor :type Actor%20Object%20Reference))
  ;[0.6445 1 0.1096] CheckCoins
  (Development|PrintString "Collision" true true "(R=0.000000,G=1.000000,B=0.167000,A=1.000000)")
  (if (Actor|ActorHasTag OtherActor "Player")
    (if (>= (Variables|/Game/Project/Blueprints/MYFirstPC.MYFirstPC_C|GetCoins (Variables|Default|GetCharacter)) (Variables|Default|GetMinCoins))
      (|CallParentFunction OtherActor))))

(event EventTick
  (params (DeltaSeconds :type Float%20%28single-precision%29))
  (|CallParentFunction DeltaSeconds) ; This node is disabled and will not be called.\nDrag off pins to build functionality.
)

(fn ConstructionScript
  (|CallParentFunction))