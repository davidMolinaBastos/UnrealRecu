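; DoorKey_Blueprint is a key-gated actor, apparently a door, that requires the player to hold a minimum number of keys.
; On BeginPlay it shows MinKey on its Number text.
; On overlap with an actor tagged Player, it calls the parent's overlap logic only if Character.Keys meets MinKey, with debug prints.
; A DoorKey widget creation branch is left unconnected and never runs.
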(event EventBeginPlay
  ;[1 1 1] Create Widget
  (Rendering|Components|TextRender|SetText (Variables|Default|GetNumber) (Utilities|Text|ToText(Integer) (Variables|Default|GetMinKey)))
  (|CallParentFunction))

(event Collision|EventActorBeginOverlap
  (params (OtherActor :type Actor%20Object%20Reference))
  (bind _character (Variables|Default|GetCharacter))
  (bind _keys (Variables|/Game/Project/Blueprints/MYFirstPC.MYFirstPC_C|GetKeys _character))
  ;[0 0.8542 1] Check Keys
  (Development|PrintString "Collision" true true "(R=0.000000,G=1.000000,B=0.167000,A=1.000000)")
  (if (Actor|ActorHasTag OtherActor "Player")
    (if (>= _keys (Variables|Default|GetMinKey))
      (Development|PrintString (Utilities|String|ToString(Integer) _keys))
      (|CallParentFunction OtherActor))))

(event EventTick
  (params (DeltaSeconds :type Float%20%28single-precision%29))
  (|CallParentFunction DeltaSeconds) ; This node is disabled and will not be called.\nDrag off pins to build functionality.
)

(fn ConstructionScript
  (|CallParentFunction))