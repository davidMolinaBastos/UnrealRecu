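; Sliding door Blueprint that rises while an actor tagged Player overlaps it and lowers when that actor leaves.
; BeginPlay records the starting height and an upper limit above it, and overlap events toggle the Open flag.
; Tick moves the door toward the matching limit without sweep, using CalculateSpeed, which adds delta seconds to the step rather than multiplying, so speed depends on frame rate.
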(event EventBeginPlay
  ;[1 0.8515 0.06772] SetVariables
  (bind _output_get (Variables|Default|SetStartZ (.Z (Math|Vector|BreakVector (Transformation|GetActorLocation)))))
  (bind _output_get_2 (Variables|Default|SetEndZ (+ _output_get 3e+02)))
  (Development|PrintString (Utilities|String|ToString(Float) _output_get_2))
  (Development|PrintString (Utilities|String|ToString(Float) (Variables|Default|GetStartZ))))

(event Collision|EventActorBeginOverlap
  (params (OtherActor :type Actor%20Object%20Reference))
  ;[1 0.1601 0.02034] DetectPlayer
  (Development|PrintString (Utilities|String|ToString(Name) (Utilities|Array|Get(acopy) (Variables|/Script/Engine.Actor|GetTags OtherActor))))
  (if (Actor|ActorHasTag OtherActor "Player")
    (Variables|Default|SetOpen true)))

(event EventTick
  (params (DeltaSeconds :type Float%20%28single-precision%29))
  ;[0.03709 0.498 1] MoveDoor
  (if (Variables|Default|GetOpen)
    (if (< (.Z (Math|Vector|BreakVector (Transformation|GetActorLocation))) (Variables|Default|GetEndZ))
      (bind _returnvalue (CallFunction|CalculateSpeed 1e+01))
      (Transformation|SetActorLocation _returnvalue false false))
    (elif (> (.Z (Math|Vector|BreakVector (Transformation|GetActorLocation))) (Variables|Default|GetStartZ))
      (bind _returnvalue_2 (CallFunction|CalculateSpeed -1e+01))
      (Transformation|SetActorLocation _returnvalue_2 false false))))

(event Collision|EventActorEndOverlap
  (params (OtherActor :type Actor%20Object%20Reference))
  ;[1 0.1601 0.02034] DetectPlayer
  (if (Actor|ActorHasTag OtherActor "Player")
    (Variables|Default|SetOpen false)))

(fn ConstructionScript)

(fn CalculateSpeed
  (params (Speed :type Float%20%28single-precision%29))
  (return (+ (Transformation|GetActorLocation) (Math|Vector|MakeVector 0.0 0.0 (+ (Utilities|Time|GetWorldDeltaSeconds) Speed)))))